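; Croissant cafe product actor whose visibility follows the player character's stock count at a fixed index in KafeUrunStoklar.
; Every Tick, it compares that stock to a per-instance threshold parsed from its fifth actor tag.
; Below the threshold, actors tagged "Silinebilir" are hidden without collision; otherwise they show, and a visibility tag mirrors the state.
; The StokAzalt event decrements the shared stock by one.
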(event Custom|Stok%20Azalt
  (CallFunction|StokAzalt 5))

(event EventTick
  (params (DeltaSeconds :type Float%20%28single-precision%29))
  (CallFunction|StokSettings 5))

(fn ConstructionScript)

(fn StokAzalt
  (params (StokIndex :type Integer))
  (bind _asfirst_person_character (Utilities|Casting|CastToFirstPersonCharacter (Game|GetPlayerCharacter 0)))
  (Utilities|Array|SetArrayElem (Variables|/Game/FirstPersonBP/Blueprints/FirstPersonCharacter.FirstPersonCharacter_C|GetKafeUrunStoklar _asfirst_person_character) StokIndex (- (Utilities|Array|Get(acopy) (Variables|/Game/FirstPersonBP/Blueprints/FirstPersonCharacter.FirstPersonCharacter_C|GetKafeUrunStoklar _asfirst_person_character) StokIndex) 1)))

(fn StokSettings
  (params (StokIndex :type Integer))
  (bind _self self)
  (bind _self_2 self)
  (bind _staticmeshcomponent (Variables|Debug|GetStaticMeshComponent))
  (bind _tags (Variables|Actor|GetTags _self))
  (bind _asfirst_person_character (Utilities|Casting|CastToFirstPersonCharacter (Game|GetPlayerCharacter 0)))
  (if (>= (Utilities|Array|Get(acopy) (Variables|/Game/FirstPersonBP/Blueprints/FirstPersonCharacter.FirstPersonCharacter_C|GetKafeUrunStoklar _asfirst_person_character) StokIndex) (Math|Conversions|ToInteger(Byte) (Utilities|String|ToString(Name) (Utilities|Array|Get(acopy) (Variables|Actor|GetTags self) 4))))
    (Rendering|SetActorHiddenInGame _self_2 false :!label _label)
    (Utilities|Array|SetArrayElem _tags 3 "Görünür")
    (Collision|SetCollisionEnabled _staticmeshcomponent "QueryAndPhysics")
    (elif (Actor|ActorHasTag self "Silinebilir")
      (Rendering|SetActorHiddenInGame _self_2 true)
      (Utilities|Array|SetArrayElem _tags 3 "Görünmez")
      (Collision|SetCollisionEnabled _staticmeshcomponent "NoCollision")
      (else
        (goto _label)))))